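; Enemy AI controller that provides chase and melee-style attack actions against the player; its own event graph is empty.
; MoveToPlayer snaps the pawn's rotation toward player 0, then uses SimpleMoveToLocation to head for that player's current location.
; AttackPlayer finds BP_ThirdPersonCharacter by class and asks whether it can block, then triggers either its block or its damage function.
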(event `self.ReceiveTick`
  (params (DeltaSeconds :type "Float (single-precision)")))

(fn `Attack Player`
  (params (Damage :type "Float (double-precision)"))
  (bind _returnvalue (`GameplayStatics.GetActorOfClass` "/Game/Blueprints/Player/Blueprints/BP_ThirdPersonCharacter.BP_ThirdPersonCharacter_C"))
  (bind (_canthrowspell _blockattack) (`/Game/Blueprints/Player/Blueprints/BP_ThirdPersonCharacter.CanBlockAttack` _returnvalue))
  (if _blockattack
    (`/Game/Blueprints/Player/Blueprints/BP_ThirdPersonCharacter.BlockAttack` _returnvalue)
    (else
      (`/Game/Blueprints/Player/Blueprints/BP_ThirdPersonCharacter.DamagePlayer` _returnvalue Damage))))

(fn `MoveToPlayer`
  (`self.K2_SetActorRotation` (`self.K2_GetPawn`) (`KismetMathLibrary.FindLookAtRotation` (`self.K2_GetActorLocation` (`self.K2_GetPawn`)) (`self.K2_GetActorLocation` (`GameplayStatics.GetPlayerCharacter` 0))) false)
  (if true
    (`AIBlueprintHelperLibrary.SimpleMoveToLocation` self (`self.K2_GetActorLocation` (`GameplayStatics.GetPlayerCharacter` 0)))))

(fn `UserConstructionScript`)