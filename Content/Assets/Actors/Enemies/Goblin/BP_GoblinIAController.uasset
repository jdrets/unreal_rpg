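; AI controller for the Goblin enemy, providing chase and attack functions without a behavior tree or active event logic of its own.
; MoveToPlayer snaps the pawn to face the player, then issues a simple navigation move to the supplied target, stopping once within close range of the player.
; AttackPlayer finds the third-person character by class and passes damage to it, with no range check.
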(event `self.ReceiveTick`
  (params (DeltaSeconds :type "Float (single-precision)")))

(fn `Attack Player`
  (params (Damage :type "Float (double-precision)"))
  (bind _returnvalue (`GameplayStatics.GetActorOfClass` "/Game/ThirdPerson/Blueprints/BP_ThirdPersonCharacter.BP_ThirdPersonCharacter_C"))
  (`/Game/ThirdPerson/Blueprints/BP_ThirdPersonCharacter.DamagePlayer` _returnvalue Damage))

(fn `MoveToPlayer`
  (params (TargetLocation :type "Vector Structure"))
  (`self.K2_SetActorRotation` (`self.K2_GetPawn`) (`KismetMathLibrary.FindLookAtRotation` (`self.K2_GetActorLocation` (`self.K2_GetPawn`)) (`self.K2_GetActorLocation` (`GameplayStatics.GetPlayerCharacter` 0))) false)
  (if (> (`KismetMathLibrary.VSize` (- (`self.K2_GetActorLocation` (`self.K2_GetPawn`)) (`self.K2_GetActorLocation` (`GameplayStatics.GetPlayerCharacter` 0)))) 150.0)
    (`AIBlueprintHelperLibrary.SimpleMoveToLocation` self TargetLocation)
    (else
      (`self.StopMovement`))))

(fn `UserConstructionScript`)