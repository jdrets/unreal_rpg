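; BP_EnemyBase is an enemy character base that chases and attacks the player and takes damage.
; Each tick, overlap boxes decide whether its AI controller pursues or stops, and trigger delayed attacks that set melee or random spell flags.
; Damage plays melee or supplied spell effects; at zero health movement and collision stop, and the actor is destroyed after a delay.
; Hovering the cursor over TargetBox shows a health bar widget.
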(event `Receive Damage`
  (params (Damage :type "Float (double-precision)") (attackType :type String) (particleEffect :type "ParticleSystem Object Reference"))
  (bind _vfx_receivespell (`self.VFX_ReceiveSpell`))
  ;[0.9786 0.315 1] Receive damage
  (if (not (<= (`self.Health`) 0.0))
    (bind _output_get (set `self.Health` (- (`self.Health`) Damage)))
    (if (== "melee" attackType)
      (`ActorComponent.Activate` (`self.VFX_HitEffect`) true)
      (else
        (`ParticleSystemComponent.SetTemplate` _vfx_receivespell particleEffect)
        (`ActorComponent.Activate` _vfx_receivespell true)))
    (if (<= _output_get 0.0)
      (`CharacterMovementComponent.SetMovementMode` (`self.CharacterMovement`) "MOVE_None" 0)
      (`PrimitiveComponent.SetCollisionEnabled` (`self.CapsuleComponent`) "NoCollision")
      (set `self.IsDead` true)
      (`KismetSystemLibrary.Delay` 10.0)
      (`self.K2_DestroyActor`))))

(event `Get player reference`
  ;[1 1 1] Get player reference
  (bind _returnvalue (`GameplayStatics.GetActorOfClass` "/Game/ThirdPerson/Blueprints/BP_ThirdPersonCharacter.BP_ThirdPersonCharacter_C"))
  (set `self.PlayerReference` _returnvalue))

(event `GetIAControllerReference`
  ;[1 1 1] Get controller reference
  (bind _asbp_enemy_iacontroller (cast `/Game/Assets/Actors/Enemies/BP_EnemyIAController` (`AIBlueprintHelperLibrary.GetAIController` self)))
  (set `self.AIControllerReference` _asbp_enemy_iacontroller))

(event `Move`
  (bind _aicontrollerreference (`self.AIControllerReference`))
  ;[0.4989 0.6101 1] Movement
  (bind _isoverlap (`self.IsPlayerOnVisibleRadio`))
  (if _isoverlap
    (bind _canmove (`self.CanMoveToPlayer`))
    (if _canmove
      (`/Game/Assets/Actors/Enemies/BP_EnemyIAController.MoveToPlayer` _aicontrollerreference)
      (else
        (`Controller.StopMovement` _aicontrollerreference)))))

(event `self.ReceiveBeginPlay`
  ;[1 0.8248 0.5249] Consstructor
  (`self.Get player reference`)
  (`self.GetIAControllerReference`))

(event `DetectToAttack`
  ;[0.5561 1 0.3524] Detect to attack
  (bind _canattack (`self.CanAttack`))
  (if _canattack
    (`KismetSystemLibrary.Delay` 0.5)
    (`self.AttackPlayer`)))

(event `self.ReceiveTick`
  (params (DeltaSeconds :type "Float (single-precision)"))
  ;[1 0.8248 0.5249] Consstructor
  (`|ExecutionSequence`
    (:`then_0`
      (`self.Move`))
    (:`then_1`
      (`self.DetectToAttack`))))

(event `self.TargetBox.OnBeginCursorOver`
  (params (TouchedComponent :type "PrimitiveComponent Object Reference"))
  ;[1 1 1] Barra de vida HUD
  (if (not (`self.IsDead`))
    (`/Engine/EditorBlueprintResources/StandardMacros.IsValid` (`self.EnemyHealthWidget`)
      (:`Is Not Valid`
        (bind _returnvalue (`|CreateWidget` "/Game/Assets/Actors/Enemies/W_EnemyHealthBar.W_EnemyHealthBar_C" null self))
        (`UserWidget.AddToViewport` _returnvalue 0)
        (set `self.EnemyHealthWidget` _returnvalue)))))

(event `self.TargetBox.OnEndCursorOver`
  (params (TouchedComponent :type "PrimitiveComponent Object Reference"))
  (bind _enemyhealthwidget (`self.EnemyHealthWidget`))
  ;[1 1 1] Barra de vida HUD
  (`/Engine/EditorBlueprintResources/StandardMacros.IsValid` _enemyhealthwidget :!label _label
    (:`Is Valid`
      (`Widget.RemoveFromParent` _enemyhealthwidget)
      (set `self.EnemyHealthWidget` null))))

(event `self.ReceiveDestroyed`
  ;[1 1 1] Barra de vida HUD
  (goto _label))

(fn `AttackPlayer`
  (if (`self.CanSpelling`)
    (if (`KismetMathLibrary.RandomBool`)
      (set `self.IsSpelling` true)
      (else
        (set `self.IsAttacking` true)))
    (else
      (set `self.IsAttacking` true))))

(fn `CanAttack`
  (returns (CanAttack :type Boolean))
  (locals (NewLocalVar :type Boolean))
  (return (and (not (`self.IsDead`)) (not (`self.IsAttacking`)) (not (`self.IsSpelling`)) (`PrimitiveComponent.IsOverlappingComponent` (`self.AttackBox`) (`Character.CapsuleComponent` (`self.PlayerReference`))))))

(fn `CanMoveToPlayer`
  (returns (CanMove :type Boolean))
  (return (and (and (and (not (`self.IsDead`)) (not (`self.IsAttacking`))) (not (`self.IsSpelling`))) (not (`PrimitiveComponent.IsOverlappingComponent` (`self.AttackBox`) (`Character.CapsuleComponent` (`self.PlayerReference`)))))))

(fn `IsPlayerOnVisibleRadio`
  (returns (IsOverlap :type Boolean))
  (locals (IsOverlappingPlayer :type Boolean))
  (for _array_element (`PrimitiveComponent.GetOverlappingActors` (`self.VisionBox`) "/Game/ThirdPerson/Blueprints/BP_ThirdPersonCharacter.BP_ThirdPersonCharacter_C")
    (bind _asbp_third_person_character (cast `/Game/ThirdPerson/Blueprints/BP_ThirdPersonCharacter` _array_element))
    (`/Engine/EditorBlueprintResources/StandardMacros.IsValid` _asbp_third_person_character
      (:`Is Valid`
        (set `local.IsOverlappingPlayer` true))
      (:`Is Not Valid`
        (set `local.IsOverlappingPlayer` false))))
  (return (`local.IsOverlappingPlayer`)))

(fn `UserConstructionScript`)