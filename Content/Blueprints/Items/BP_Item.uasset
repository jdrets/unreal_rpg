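; BP_Item is an item actor that shows its name in a floating label while the cursor hovers over it.
; Cursor-over events on TargetBox create a W_ItemDisplayName widget from the Item's Name and remove it when the cursor leaves.
; Tick repositions the widget just above the mouse position, and Destroyed removes any label still on screen.
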(event `self.ReceiveDestroyed`
  (bind _displaynamewidget (`self.DisplayNameWidget`))
  ;[1 1 1] On destroy item
  (if (`KismetSystemLibrary.IsValid` _displaynamewidget)
    (`Widget.RemoveFromParent` _displaynamewidget)
    (set `self.DisplayNameWidget` null)))

(event `self.ReceiveTick`
  (params (DeltaSeconds :type "Float (single-precision)"))
  (bind (_locationx _locationy) (`PlayerController.GetMousePosition` (`GameplayStatics.GetPlayerController` 0)))
  ;[1 1 1] Mover display name segun el mouse
  (`|ExecutionSequence`
    (:`then_0`
      (if (`KismetSystemLibrary.IsValid` (`self.DisplayNameWidget`))
        (`UserWidget.SetPositionInViewport` (`self.DisplayNameWidget`) (`KismetMathLibrary.MakeVector2D` _locationx (- _locationy 32.0)) true)))))

(event `self.TargetBox.OnBeginCursorOver`
  (params (TouchedComponent :type "PrimitiveComponent Object Reference"))
  ;[1 1 1] Dibujar display name widget
  (if (not (`KismetSystemLibrary.IsValid` (`self.DisplayNameWidget`)))
    (bind _returnvalue (`|CreateWidget` "/Game/Blueprints/Items/W_ItemDisplayName.W_ItemDisplayName_C" null (`KismetStringLibrary.Conv_NameToString` (`.name_6_FFF8A70E46EA664B6EFB4BA901737094` (break `/Game/Blueprints/Items/ST_Item` (`self.Item`))))))
    (bind _output_get (set `self.DisplayNameWidget` _returnvalue))
    (`UserWidget.AddToViewport` _output_get 0)))

(event `self.TargetBox.OnEndCursorOver`
  (params (TouchedComponent :type "PrimitiveComponent Object Reference"))
  (bind _displaynamewidget (`self.DisplayNameWidget`))
  ;[1 1 1] Destruir display name
  (if (`KismetSystemLibrary.IsValid` _displaynamewidget)
    (`Widget.RemoveFromParent` _displaynamewidget)
    (set `self.DisplayNameWidget` null)))

(fn `UserConstructionScript`)