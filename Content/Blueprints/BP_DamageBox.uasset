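; BP_DamageBox is a hazard actor that periodically damages the player while something overlaps it.
; Begin and end overlap events toggle a collision flag for any actor, without checking which one entered.
; Tick calls DamagePlayer on the first BP_ThirdPersonCharacter found, then uses a CanDamage gate and a two-second Delay as a cooldown before the next hit.
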(event `self.ReceiveActorEndOverlap`
  (params (OtherActor :type "Actor Object Reference"))
  ;[1 1 1] C olision event
  (set `self.isCollision` false))

(event `self.ReceiveActorBeginOverlap`
  (params (OtherActor :type "Actor Object Reference"))
  ;[1 1 1] C olision event
  (set `self.isCollision` true))

(event `self.ReceiveTick`
  (params (DeltaSeconds :type "Float (single-precision)"))
  ;[1 0.3583 0.349] Damage player
  (if (`self.isCollision`)
    (if (`self.canDamage`)
      (set `self.canDamage` false)
      (bind _returnvalue (`GameplayStatics.GetActorOfClass` "/Game/ThirdPerson/Blueprints/BP_ThirdPersonCharacter.BP_ThirdPersonCharacter_C"))
      (`/Game/ThirdPerson/Blueprints/BP_ThirdPersonCharacter.DamagePlayer` _returnvalue (`self.Damage`))
      (`KismetSystemLibrary.LogString` "Danio")
      (`KismetSystemLibrary.Delay` 2.0)
      (set `self.canDamage` true))))

(fn `UserConstructionScript`)